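; BP_Drink is a drink in The Outer Bar that tracks how much it has been shaken and stirred.
; Each tick it compares shake and stir values, which are not set in this graph, against fixed thresholds.
; Crossing a threshold increments the matching counter, plays a right-hand haptic effect and resets that value.
; Reaching the stir count target only prints a debug message.
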(event Custom|checkShake
  ;[0.15 0.15 0.15 0.5] Each frame, check shake val. If above threshold, increment shaken and play haptic feedback
  (if (>= (Variables|Default|GetshakeVal) 3.0)
    (Math|Integer|IncrementInt (Variables|Default|GetShaken)
      (:%20%20
        (Class|PlayerController|PlayHapticEffect (Game|GetPlayerController 0) "/Game/VRTemplate/Haptics/PistolFireHapticEffect.PistolFireHapticEffect" "Right" 1.0 false)
        (Variables|Default|SetshakeVal 0.0)))))

(event Custom|checkStir
  ;[0.15 0.15 0.15 0.5] Each frame, check shake val. If above threshold, increment shaken and play haptic feedback
  (if (>= (Variables|Default|GetstirVal) 2.0)
    (Math|Integer|IncrementInt (Variables|Default|GetStirred)
      (:%20%20
        (Class|PlayerController|PlayHapticEffect (Game|GetPlayerController 0) "/Game/VRTemplate/Haptics/PistolFireHapticEffect.PistolFireHapticEffect" "Right" 1.0 false)
        (Variables|Default|SetstirVal 0.0)
        (if (>= (Variables|Default|GetStirred) 2)
          (Development|PrintString "Stir done"))))))

(event EventBeginPlay)

(event Collision|EventActorBeginOverlap
  (params (OtherActor :type Actor%20Object%20Reference)))

(event EventTick
  (params (DeltaSeconds :type Float%20%28single-precision%29))
  (CallFunction|CheckSHake)
  (CallFunction|CheckStir))

(fn ConstructionScript)
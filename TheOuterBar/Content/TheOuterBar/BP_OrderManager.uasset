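; Order manager for a VR bartending game that generates random NPC drink orders and pays the player for served drinks.
; CreateOrder rolls a recipe, two distinct ingredients, garnish, stir, shake and glass type, stores it by NPC, and updates that NPC's order widget.
; CompleteOrder deducts from a tip score for ingredient, amount, stir, shake and glass mismatches, ignoring garnish.
; The score scales the money added to VRPawn, then resets.
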(event Custom|Create%20Order
  (params (NPC%20Ref :type Zeno%20NPC%20Blueprint%20Object%20Reference))
  (bind _drinkchosenname (Variables|Default|GetDrinkChosenName))
  (bind _widget (Variables|/Game/Characters/NPCs/Zenomorph/ZenoNPCBlueprint.ZenoNPCBlueprint_C|GetWidget NPC%20Ref))
  ;[0.15 0.15 0.15 0.5 40] Make Order
  (bind _ingredient (CallFunction|PickRandomIngredientAmount))
  (bind _ingredient_2 (CallFunction|PickRandomIngredientAmount :!label _label))
  (if (Utilities|Enum|Equal(Enum) (.IngredientName (Utilities|Struct|BreakIngredientEntry _ingredient)) (.IngredientName (Utilities|Struct|BreakIngredientEntry _ingredient_2)))
    (goto _label)
    (else
      (bind _output_get (Variables|Default|SetIngredient2Chosen _ingredient_2))
      (bind _ingredient_3 (CallFunction|PickRandomIngredientAmount))
      (bind _returnvalue (Utilities|Array|Add (Variables|Default|GetActiveOrders) (Utilities|Struct|MakeFOrderInfo NPC%20Ref (Utilities|Array|Get(acopy) _drinkchosenname (.OutIndex (Utilities|Array|Random _drinkchosenname))) _ingredient _output_get _ingredient_3 (Math|Random|RandomIntegerinRange 1 4) (Math|Random|RandomIntegerinRange 1 4) (Math|Random|RandomBool))))
      (bind _output_get_2 (Variables|Default|SetNewOrderIndex _returnvalue))
      (Math|Integer|IncrementInt (Variables|Default|GetNextOrderId)
        (:%20%20
          (Utilities|Map|Add (Variables|Default|GetNPCToOrder) NPC%20Ref _output_get_2)
          (bind _asdrink_order_display (Utilities|Casting|CastToDrinkOrderDisplay (UserInterface|GetWidget _widget)))
          (Default|UpdateText _asdrink_order_display (Utilities|Struct|MakeFOrderInfo NPC%20Ref (Utilities|Array|Get(acopy) _drinkchosenname (.OutIndex (Utilities|Array|Random _drinkchosenname))) _ingredient _output_get _ingredient_3 (Math|Random|RandomIntegerinRange 1 4) (Math|Random|RandomIntegerinRange 1 4) (Math|Random|RandomBool)))
          (Rendering|SetVisibility _widget true true))))))

(event Custom|Complete%20Order
  (params (NPC%20Ref :type Zeno%20NPC%20Blueprint%20Object%20Reference) (Drink :type BP%20Drink%201%20Object%20Reference))
  (bind _activeorders (Variables|Default|GetActiveOrders))
  (bind _npctoorder (Variables|Default|GetNPCToOrder))
  (bind _drinkstuff (Variables|/Game/TheOuterBar/BP_Drink1.BP_Drink1_C|GetDrinkStuff Drink))
  (bind _value (Utilities|Map|Find _npctoorder NPC%20Ref))
  (bind _output (Utilities|Array|Get(acopy) _activeorders _value))
  (bind (_npcref _drinkrecipechosen _ingredients1 _ingredient2 _garnish _stir _shake _glasstype) (Utilities|Struct|BreakFOrderInfo _output))
  ;[0.15 0.15 0.15 0.5 40] CompleteOrder
  (bind _match (CallFunction|IngredientComparison (.ingredients1 _drinkstuff) _ingredients1))
  (if _match
    (bind _match_2 (CallFunction|IngredientComparison (.ingredient2 _drinkstuff) _ingredient2 :!label _label))
    (if _match_2
      _
      (else
        (Variables|Default|SetMinTip (- (Variables|Default|GetMinTip) 2e+01))))
    (else
      (bind _match_3 (CallFunction|IngredientComparison (.ingredients1 _drinkstuff) _ingredient2))
      (if _match_3
        _
        (else
          (Variables|Default|SetMinTip (- (Variables|Default|GetMinTip) 1e+01))))
      (bind _match_4 (CallFunction|IngredientComparison (.ingredient2 _drinkstuff) _ingredients1))
      (if _match_4
        _
        (else
          (goto _label)))))
  (Variables|Default|SetMinTip (+ (* (Math|Integer|Absolute(Integer) (- (.stir _drinkstuff) _stir)) -1) (Variables|Default|GetMinTip)))
  (bind _output_get (Variables|Default|SetMinTip (+ (* (Math|Integer|Absolute(Integer) (- (.shake _drinkstuff) _shake)) -1) (Variables|Default|GetMinTip))))
  (if (== (.glasstype _drinkstuff) _glasstype)
    _
    (else
      (Variables|Default|SetMinTip (- _output_get 2e+01))))
  (bind _output_get_2 (Variables|Default|SetMinTip (/ (Variables|Default|GetMinTip) 1e+02)))
  (bind _asvrpawn (Utilities|Casting|CastToVRPawn (Game|Player|GetPlayerPawn 0)))
  (Math|Float|IncrementFloat (Variables|/Game/VRTemplate/Blueprints/VRPawn.VRPawn_C|GetNumDrinks _asvrpawn)
    (:%20%20
      (Variables|/Game/VRTemplate/Blueprints/VRPawn.VRPawn_C|SetMoney _asvrpawn (+ (* 25.0 _output_get_2) (Variables|/Game/VRTemplate/Blueprints/VRPawn.VRPawn_C|GetMoney _asvrpawn)))
      (Variables|Default|SetMinTip 1e+02))))

(event Custom|OrderUISetup
  ;[0.15 0.15 0.15 0.5 40] UI for Order
)

(event EventBeginPlay)

(event Collision|EventActorBeginOverlap
  (params (OtherActor :type Actor%20Object%20Reference)))

(event EventTick
  (params (DeltaSeconds :type Float%20%28single-precision%29)))

(fn ConstructionScript)

(fn PickRandomIngredientAmount
  (bind _ingredients_chosen (Variables|Default|GetIngredients%20Chosen))
  (return (Utilities|Struct|MakeIngredientEntry (.IngredientName (Utilities|Struct|BreakIngredientEntry (Utilities|Array|Get(acopy) _ingredients_chosen (.OutIndex (Utilities|Array|Random _ingredients_chosen))))) (Math|Random|RandomIntegerinRange 1 4))))

(fn IngredientComparison
  (params (IngredientCompare1 :type Ingredient%20Entry%20Structure) (IngredientCompare2 :type Ingredient%20Entry%20Structure))
  (bind _returnvalue (Utilities|Enum|Equal(Enum) (.ingredientname IngredientCompare1) (.ingredientname IngredientCompare2)))
  (if _returnvalue
    (Variables|Default|SetMinTip (+ (Variables|Default|GetMinTip) (* (Math|Integer|Absolute(Integer) (- (.requiredamount IngredientCompare1) (.requiredamount IngredientCompare2))) -1)))
    (return _returnvalue)))
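; Gesture component that detects shaking, stirring and pouring with a held bar tool and writes progress to its drink instance.
; While tracking, Tick derives the tracked component's velocity and speed, then runs three handlers filtered by held actor type.
; Shake and stir add frame time above speed thresholds; pour uses tilt-angle hysteresis to scale flow while overlapping.
; The angle-accumulating circular stir detection is disconnected, leaving its stir context unused.
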(event Custom|HandlePour
  (bind _asgrabbable_shaker (Utilities|Casting|CastToGrabbable_Shaker (Variables|Default|GetCurrentHeldActor)))
  (bind _output_get (Variables|Default|SetHandUpWS (Math|Vector|GetUpVector (Variables|Default|GetTrackedComponent))))
  (Variables|Default|SetangleDeg (Math|Trig|RadiansToDegrees (Math|Trig|Acos(Degrees) (Math|Vector|DotProduct "0.000000,1.000000,0.000000" _output_get))))
  (if (and (not (Variables|Default|GetbIsPouring)) (>= (Variables|Default|GetangleDeg) (Variables|Default|GetPourStartAngleDeg)))
    (Variables|Default|SetbIsPouring true)
    (elif (and (Variables|Default|GetbIsPouring) (<= (Variables|Default|GetangleDeg) (Variables|Default|GetPourStopAngleDeg)))
      (Variables|Default|SetbIsPouring false)
      (elif (Variables|Default|GetbIsPouring)
        (bind _output_get_2 (Variables|Default|SettiltRange (- (Variables|Default|GetMaxPourAngleDeg) (Variables|Default|GetPourStartAngleDeg))))
        (Variables|Default|SetCurrentPourStrength%20 (/ (Math|Float|Clamp(Float) (- (Variables|Default|GetangleDeg) (Variables|Default|GetPourStartAngleDeg)) 0.0 _output_get_2) (Variables|Default|GettiltRange)))
        (if (Variables|Default|Getoverlapping)
          (Variables|/Game/TheOuterBar/BP_Drink1.BP_Drink1_C|SetpouredVal (Variables|/Game/VRTemplate/Blueprints/Grabbable_Shaker.Grabbable_Shaker_C|GetcurrDrinkInst _asgrabbable_shaker) (+ (* (Variables|Default|GetPourFlowRate) (Variables|Default|GetCurrentPourStrength%20) (Variables|Default|GetDelta%20Seconds)) (Variables|/Game/TheOuterBar/BP_Drink1.BP_Drink1_C|GetpouredVal (Variables|/Game/VRTemplate/Blueprints/Grabbable_Shaker.Grabbable_Shaker_C|GetcurrDrinkInst _asgrabbable_shaker)))))))))

(event Custom|HandleShake
  ;[0.15 0.15 0.15 0.5] Update Status towards shake gesture
  (bind _asgrabbable_shaker (Utilities|Casting|CastToGrabbable_Shaker (Variables|Default|GetCurrentHeldActor)))
  (bind _shakeval (CallFunction|GetAccumulatedShake))
  (bind _asbp_drink_1 (Utilities|Casting|CastToBP_Drink1 (Variables|/Game/VRTemplate/Blueprints/Grabbable_Shaker.Grabbable_Shaker_C|GetcurrDrinkInst _asgrabbable_shaker)))
  (Variables|/Game/TheOuterBar/BP_Drink1.BP_Drink1_C|SetshakeVal _asbp_drink_1 (+ (Variables|/Game/TheOuterBar/BP_Drink1.BP_Drink1_C|GetshakeVal _asbp_drink_1) _shakeval)))

(event Custom|HandleStir
  ;[0.15 0.15 0.15 0.5] Update Status towards shake gesture
  (bind _asgrabbable_spoon (Utilities|Casting|CastToGrabbable_Spoon (Variables|Default|GetCurrentHeldActor)))
  (if (Variables|/Game/VRTemplate/Blueprints/Grabbable_Spoon.Grabbable_Spoon_C|GetspoonInCup _asgrabbable_spoon)
    (bind _shakeval (CallFunction|GetAccumulatedStir))
    (Utilities|IsValid (Variables|/Game/VRTemplate/Blueprints/Grabbable_Spoon.Grabbable_Spoon_C|GetcurrDrinkInst _asgrabbable_spoon)
      (:Is%20Valid
        (Variables|/Game/TheOuterBar/BP_Drink1.BP_Drink1_C|SetstirVal (Variables|/Game/VRTemplate/Blueprints/Grabbable_Spoon.Grabbable_Spoon_C|GetcurrDrinkInst _asgrabbable_spoon) (+ (Variables|/Game/TheOuterBar/BP_Drink1.BP_Drink1_C|GetstirVal (Variables|/Game/VRTemplate/Blueprints/Grabbable_Spoon.Grabbable_Spoon_C|GetcurrDrinkInst _asgrabbable_spoon)) _shakeval)))
      (:Is%20Not%20Valid
        (Development|PrintString "inst not valid")))))

(event EventBeginPlay)

(event EventTick
  (params (DeltaSeconds :type Float%20%28single-precision%29))
  (bind _trackedcomponent (Variables|Default|GetTrackedComponent))
  (bind _returnvalue (Transformation|GetWorldLocation _trackedcomponent))
  ;[0.15 0.15 0.15 0.5] Get Speed and other data from controller each tick
  (Variables|Default|SetDelta%20Seconds DeltaSeconds)
  (if (Variables|Default|GetbIsTracking)
    (Variables|Default|SetVelocity (/ (- _returnvalue (Variables|Default|GetLastLocation)) (Variables|Default|GetDelta%20Seconds)))
    (Variables|Default|SetSpeed (Math|Vector|VectorLength (/ (- _returnvalue (Variables|Default|GetLastLocation)) (Variables|Default|GetDelta%20Seconds))))
    (Variables|Default|SetLastLocation _returnvalue)
    (Utilities|IsValid (Variables|Default|GetCurrentHeldActor)
      (:Is%20Valid
        (CallFunction|HandleShake)
        (CallFunction|HandleStir)
        (CallFunction|HandlePour)))))

(fn StartTracking
  (params (HeldActor :type Actor%20Object%20Reference))
  (Variables|Default|SetbIsTracking true)
  (Variables|Default|SetCurrentHeldActor HeldActor)
  (Variables|Default|SetLastLocation (Transformation|GetActorLocation (Components|GetOwner)))
  (Variables|Default|SetVelocity "0, 0, 0")
  (Variables|Default|SetSpeed 0.0)
  (Variables|Default|SetShakeAccumulatedTime 0.0)
  (Variables|Default|SetbHasLastShakeDir false)
  (Variables|Default|SetAccumulatedStirAngle 0.0)
  (Variables|Default|SetbHasLastLocalDir false))

(fn StopTracking
  (Variables|Default|SetbIsTracking false)
  (Variables|Default|SetCurrentHeldActor 0))

(fn SetStirContext
  (params (OriginWS :type Vector) (RadiusMin :type Float%20%28double-precision%29) (RadiusMax :type Float%20%28double-precision%29))
  (Variables|Default|SetStirOriginWS OriginWS)
  (Variables|Default|SetStirRadiusMin RadiusMin)
  (Variables|Default|SetStirRadiusMax RadiusMax)
  (Variables|Default|SetbHasStirContext true)
  (Variables|Default|SetAccumulatedStirAngle 0.0)
  (Variables|Default|SetbHasLastLocalDir false))

(fn ClearStirContext
  (Variables|Default|SetbHasStirContext false))

(fn GetAccumulatedShake
  (if (and (Variables|Default|GetbHasLastShakeDir) (> (Variables|Default|GetSpeed) (Variables|Default|GetShakeSpeedThreshold)))
    (if (< (Math|Vector|DotProduct "0, 0, 0" (Variables|Default|GetLastShakeDir)) (Variables|Default|GetMinDirectionDot))
      (return (Variables|Default|GetDelta%20Seconds))
      (else
        _))
    (else
      (Variables|Default|SetLastShakeDir "0, 0, 0")
      (Variables|Default|SetbHasLastShakeDir true)))
  (return 0.0))

(fn GetAccumulatedStir
  (if (> (Variables|Default|GetSpeed) 15.0)
    (return (Variables|Default|GetDelta%20Seconds))
    (else
      (return 0.0))))